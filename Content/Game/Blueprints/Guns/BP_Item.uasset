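; BP_Item is a pickup item Blueprint that shows an on-screen interaction prompt while a character is in pickup range.
; On range entered, it creates an Interaction widget for the character's player controller in a new screen-space, collision-free widget component.
; The component snaps to the component returned by AttachText, here the default scene root.
; On range exited, the stored component is destroyed if valid.
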(event `/Game/Game/Blueprints/Interfaces/Interact.PickUpRangeEntered`
  (params (Character :type "/Game/Game/Blueprints/Character/FirstPersonCharacter Object Reference"))
  (bind _returnvalue (`|CreateWidget` "/Game/Game/Blueprints/HUD/Interaction.Interaction_C" (cast `PlayerController` (`Pawn.GetController` Character) :!pure true)))
  (bind _returnvalue_2 (`AddComponent|NODE_AddWidgetComponent-0`))
  (bind _output_get (set `self.InteractionWidget` _returnvalue_2))
  (`WidgetComponent.SetWidget` _output_get _returnvalue)
  (`WidgetComponent.SetWidgetSpace` _output_get "Screen")
  (`WidgetComponent.SetDrawAtDesiredSize` _output_get true)
  (`PrimitiveComponent.SetCollisionEnabled` _output_get "NoCollision")
  (`SceneComponent.K2_AttachToComponent` _output_get (`self.AttachText`) "None" "SnapToTarget" "SnapToTarget" "SnapToTarget" true))

(event `/Game/Game/Blueprints/Interfaces/Interact.PickUpRangeExited`
  (bind _interactionwidget (`self.InteractionWidget`)
    (:`then`
      (`ActorComponent.K2_DestroyComponent` _interactionwidget))
    (:`else`)))

(fn `AttachText`
  (returns (AttachComponent :type "SceneComponent Object Reference"))
  (return (`self.DefaultSceneRoot`)))

(fn `UserConstructionScript`)
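; LavaFloor is a hazard actor that damages the first-person character while it stands on the lava.
; BeginPlay caches the FirstPersonCharacter, and a Box begin overlap by that character sets IsOnLava and starts a Delay loop.
; The loop calls TakeDamageFromLava on the character after each half-second wait and repeats while the flag holds.
; Any actor ending overlap with the box clears the flag.
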(event `self.ReceiveBeginPlay`
  (bind _returnvalue (`GameplayStatics.GetActorOfClass` "/Game/Game/Blueprints/Character/FirstPersonCharacter.FirstPersonCharacter_C"))
  (set `self.Character` _returnvalue))

(event `self.Box.OnComponentBeginOverlap`
  (params (OverlappedComponent :type "PrimitiveComponent Object Reference") (OtherActor :type "Actor Object Reference") (OtherComp :type "PrimitiveComponent Object Reference") (OtherBodyIndex :type Integer) (bFromSweep :type Boolean) (SweepResult :type "HitResult Structure (by ref)"))
  (bind _character (`self.Character`))
  (if (== OtherActor _character)
    (`/Engine/EditorBlueprintResources/StandardMacros.IsValid` _character
      (:`Is Valid`
        ;[1 1 1] Take damage if on lava
        (set `self.IsOnLava` true)
        (`KismetSystemLibrary.Delay` 0.5 :!label _label)
        (`/Game/Game/Blueprints/Character/FirstPersonCharacter.TakeDamageFromLava` _character)
        (if (`self.IsOnLava`)
          (goto _label))))))

(event `self.Box.OnComponentEndOverlap`
  (params (OverlappedComponent :type "PrimitiveComponent Object Reference") (OtherActor :type "Actor Object Reference") (OtherComp :type "PrimitiveComponent Object Reference") (OtherBodyIndex :type Integer))
  (set `self.IsOnLava` false))

(fn `UserConstructionScript`)
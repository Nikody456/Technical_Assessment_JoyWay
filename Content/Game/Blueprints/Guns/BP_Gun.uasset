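; BP_Gun is a gun actor that can be picked up by a character, fire bullets and reload.
; The PickUp event passes the gun to the character's own PickUp.
; Fire spawns a Bullet actor at the skeletal mesh's Muzzle socket and spends one loaded round.
; Reload refills Ammo up to AmmoSize from the MaxAmmo reserve, using whatever remains when it runs short; AttachText is an empty stub.
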(event `/Game/Game/Blueprints/Interfaces/Interact.PickUp`
  (params (Character :type "/Game/Game/Blueprints/Character/FirstPersonCharacter Object Reference"))
  (`/Game/Game/Blueprints/Character/FirstPersonCharacter.PickUp` Character self))

(fn `AttachText`
  (returns (AttachComponent :type "SceneComponent Object Reference"))
  (return null))

(fn `Fire`
  (if (> (`self.AmmoSize`) 0)
    (if (> (`self.Ammo`) 0)
      (`|SpawnActorFromClass` "/Game/Game/Blueprints/Bullets/Bullet.Bullet_C" (`SceneComponent.GetSocketTransform` (`self.SkeletalMesh`) "Muzzle" "RTS_World") "Undefined" "OverrideRootScale" null null)
      (set `self.Ammo` (- (`self.Ammo`) 1)))))

(fn `Reload`
  (if (== (`self.Ammo`) (`self.AmmoSize`))
    _
    (elif (> (- (`self.AmmoSize`) (`self.Ammo`)) (`self.MaxAmmo`))
      (set `self.Ammo` (+ (`self.Ammo`) (`self.MaxAmmo`)))
      (set `self.MaxAmmo` 0)
      (else
        (set `self.MaxAmmo` (- (`self.MaxAmmo`) (- (`self.AmmoSize`) (`self.Ammo`))))
        (set `self.Ammo` (+ (`self.Ammo`) (- (`self.AmmoSize`) (`self.Ammo`))))))))

(fn `UserConstructionScript`
  (`parent.UserConstructionScript`))
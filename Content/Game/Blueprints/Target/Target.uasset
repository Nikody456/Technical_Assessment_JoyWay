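; Target is a shootable actor that loses health when bullets hit it and destroys itself once health runs out.
; Separate Head and Body components handle overlaps, cast the other actor to Bullet, and subtract damage, with head hits costing more than body hits.
; BeginPlay also stores the first Bullet actor found in the level, though the overlap logic never reads that reference.
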(event `self.ReceiveBeginPlay`
  (bind _returnvalue (`GameplayStatics.GetActorOfClass` "/Game/Game/Blueprints/Bullets/Bullet.Bullet_C"))
  (set `self.Bullet` _returnvalue))

(event `self.Head.OnComponentBeginOverlap`
  (params (OverlappedComponent :type "PrimitiveComponent Object Reference") (OtherActor :type "Actor Object Reference") (OtherComp :type "PrimitiveComponent Object Reference") (OtherBodyIndex :type Integer) (bFromSweep :type Boolean) (SweepResult :type "HitResult Structure (by ref)"))
  (cast `/Game/Game/Blueprints/Bullets/Bullet` OtherActor)
  (set `self.Health` (- (`self.Health`) 0.2))
  (if (<= (`self.Health`) 0.0)
    (`self.K2_DestroyActor`)))

(event `self.Body.OnComponentBeginOverlap`
  (params (OverlappedComponent :type "PrimitiveComponent Object Reference") (OtherActor :type "Actor Object Reference") (OtherComp :type "PrimitiveComponent Object Reference") (OtherBodyIndex :type Integer) (bFromSweep :type Boolean) (SweepResult :type "HitResult Structure (by ref)"))
  (cast `/Game/Game/Blueprints/Bullets/Bullet` OtherActor)
  (set `self.Health` (- (`self.Health`) 0.05))
  (if (<= (`self.Health`) 0.0)
    (`self.K2_DestroyActor`)))

(fn `UserConstructionScript`)